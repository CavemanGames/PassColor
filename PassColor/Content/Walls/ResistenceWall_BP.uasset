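; ResistenceWall_BP is a wall Blueprint that gives its cube mesh a random color.
; The Construction Script creates a dynamic material instance from WallMat and stores it as WallColor.
; It rolls red, green and blue separately in tenths and writes them to the BaseColor parameter, so the color can change whenever construction reruns.
; The event graph has no active logic.
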(event EventBeginPlay)

(event Collision|EventActorBeginOverlap
  (params (OtherActor :type Actor%20Object%20Reference)))

(event EventTick
  (params (DeltaSeconds :type Float%20%28single-precision%29)))

(fn ConstructionScript
  (bind _returnvalue (Rendering|Material|CreateDynamicMaterialInstance (Variables|Default|GetCube) 0 "/Game/Walls/WallMat.WallMat" :!class /Script/Engine.PrimitiveComponent))
  (Variables|Default|SetWallColor _returnvalue)
  (Variables|Default|SetRedColor (/ (Math|Conversions|ToFloat(Integer) (Math|Random|RandomIntegerinRange 0 10)) 1e+01))
  (Variables|Default|SetGreenColor (/ (Math|Conversions|ToFloat(Integer) (Math|Random|RandomIntegerinRange 0 10)) 1e+01))
  (Variables|Default|SetBlueColor (/ (Math|Conversions|ToFloat(Integer) (Math|Random|RandomIntegerinRange 0 10)) 1e+01))
  (Rendering|Material|SetVectorParameterValue (Variables|Default|GetWallColor) "BaseColor" (Utilities|Struct|MakeLinearColor (Variables|Default|GetRedColor) (Variables|Default|GetGreenColor) (Variables|Default|GetBlueColor) 1.0) :!class /Script/Engine.MaterialInstanceDynamic))