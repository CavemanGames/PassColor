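; Colored ball actor that gets one of eight RGB color-combination sprites at random.
; The construction script switches on a random integer to set the SpriteColor sprite, with the last case sharing the default "discolors" branch.
; It then stores the chosen sprite's display name in SetedSpriteName.
; The event graph holds only disabled placeholder events, so all logic runs at construction.
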(event EventBeginPlay)

(event Collision|EventActorBeginOverlap
  (params (OtherActor :type Actor%20Object%20Reference)))

(event EventTick
  (params (DeltaSeconds :type Float%20%28single-precision%29)))

(fn ConstructionScript
  (switch int (Math|Random|RandomIntegerinRange 0 7)
    (:Default
      (Rendering|Components|Sprite|SetSprite (Variables|Default|GetSpriteColor) "/Game/Balls/Sprites/RGB_discolors_Sprite.RGB_discolors_Sprite" :!label _label))
    (:0
      (Rendering|Components|Sprite|SetSprite (Variables|Default|GetSpriteColor) "/Game/Balls/Sprites/B_color_Sprite.B_color_Sprite"))
    (:1
      (Rendering|Components|Sprite|SetSprite (Variables|Default|GetSpriteColor) "/Game/Balls/Sprites/G_color_Sprite.G_color_Sprite"))
    (:2
      (Rendering|Components|Sprite|SetSprite (Variables|Default|GetSpriteColor) "/Game/Balls/Sprites/GB_color_Sprite.GB_color_Sprite"))
    (:3
      (Rendering|Components|Sprite|SetSprite (Variables|Default|GetSpriteColor) "/Game/Balls/Sprites/R_color_Sprite.R_color_Sprite"))
    (:4
      (Rendering|Components|Sprite|SetSprite (Variables|Default|GetSpriteColor) "/Game/Balls/Sprites/RB_color_Sprite.RB_color_Sprite"))
    (:5
      (Rendering|Components|Sprite|SetSprite (Variables|Default|GetSpriteColor) "/Game/Balls/Sprites/RG_color_Sprite.RG_color_Sprite"))
    (:6
      (Rendering|Components|Sprite|SetSprite (Variables|Default|GetSpriteColor) "/Game/Balls/Sprites/RGB_colors_Sprite.RGB_colors_Sprite"))
    (:7
      (goto _label)))
  (Variables|Default|SetSetedSpriteName (Utilities|GetDisplayName (Sprite|GetSprite (Variables|Default|GetSpriteColor)))))